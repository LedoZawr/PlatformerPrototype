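; Game mode that handles respawning the player.
; Tick retries caching BP_GameInstance until the reference is valid.
; Respawn spawns a new BP_Player at SpawnTransform, possesses it and restores unpaused, game-only input with the cursor hidden.
; It then refills the health stored on the game instance, except after a fall death, where it only clears the IsDyingFromFall flag.
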(event `self.ReceiveTick`
  (params (DeltaSeconds :type "Float (single-precision)"))
  (`/Engine/EditorBlueprintResources/StandardMacros.IsValid` (`self.As BP Game Instance`)
    (:`Is Not Valid`
      (bind _asbp_game_instance (cast `/Game/Miscellaneous/BP_GameInstance` (`GameplayStatics.GetGameInstance`)))
      (set `self.As BP Game Instance` _asbp_game_instance))))

(event `Respawn`
  (bind _as_bp_game_instance (`self.As BP Game Instance`))
  (`WidgetBlueprintLibrary.SetInputMode_GameOnly` (`GameplayStatics.GetPlayerController` 0))
  (bind _returnvalue (`|SpawnActorFromClass` "/Game/Characters/BP_Player.BP_Player_C" (`self.SpawnTransform`) "AdjustIfPossibleButAlwaysSpawn" "MultiplyWithRoot" null null))
  (`Controller.Possess` (`GameplayStatics.GetPlayerController` 0) _returnvalue)
  (`GameplayStatics.SetGamePaused` false)
  (set `PlayerController.bShowMouseCursor` false (`GameplayStatics.GetPlayerController` 0))
  (if (`/Game/Miscellaneous/BP_GameInstance.IsDyingFromFall` (`self.As BP Game Instance`))
    (set `/Game/Miscellaneous/BP_GameInstance.IsDyingFromFall` false (`self.As BP Game Instance`))
    (else
      (set `/Game/Miscellaneous/BP_GameInstance.GIHeath` (`/Game/Miscellaneous/BP_GameInstance.GIMaxHealth` _as_bp_game_instance) _as_bp_game_instance))))

(fn `UserConstructionScript`)