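; BP_BlueDoor is a double door that swings open when the blue button has been pressed.
; Tick polls IsBlueBtnPressed on the cached BP_GameInstance and, while true, plays the DoorOpens timeline.
; The timeline's alpha lerps both door holders' relative rotations in opposite yaw directions, with no closing logic.
; BeginPlay also stores a BP_BlueButton reference, but the door's logic does not use it.
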(event `self.ReceiveBeginPlay`
  (bind _returnvalue (`GameplayStatics.GetActorOfClass` "/Game/Interactables/DoorsWithButtons/BP_BlueButton.BP_BlueButton_C"))
  (set `self.ButtonRef` _returnvalue)
  (bind _asbp_game_instance (cast `/Game/Miscellaneous/BP_GameInstance` (`GameplayStatics.GetGameInstance`)))
  (set `self.As BP Game Instance` _asbp_game_instance))

(event `self.ReceiveTick`
  (params (DeltaSeconds :type "Float (single-precision)"))
  (if (`/Game/Miscellaneous/BP_GameInstance.IsBlueBtnPressed` (`self.As BP Game Instance`))
    (bind (_direction _alpha) (`Timeline|DoorOpens`)
      (:`Update`
        (set `self.DoorOpenAlpha` _alpha)
        (`|ExecutionSequence`
          (:`then_0`
            (`SceneComponent.K2_SetRelativeRotation` (`self.Door1Holder`) (`KismetMathLibrary.RLerp` (struct) (struct :`Yaw` -90.0) (`self.DoorOpenAlpha`)) false false))
          (:`then_1`
            (`SceneComponent.K2_SetRelativeRotation` (`self.Door2Holder`) (`KismetMathLibrary.RLerp` (struct) (struct :`Yaw` 90.0) (`self.DoorOpenAlpha`)) false false)))))))

(fn `UserConstructionScript`)