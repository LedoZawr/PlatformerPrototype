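; BP_BlueButton is an interactable button that records a blue-button press when the player character overlaps its box.
; The overlap plays the ButtonMovement timeline, which lerps the cube's relative location along Z.
; Each timeline update also sets IsBlueBtnPressed on the BP_GameInstance cached at BeginPlay, so the pressed state lives in the game instance.
; The file has no logic to reverse the movement or clear the flag.
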(event `self.ReceiveBeginPlay`
  (bind _asbp_game_instance (cast `/Game/Miscellaneous/BP_GameInstance` (`GameplayStatics.GetGameInstance`)))
  (set `self.As BP Game Instance` _asbp_game_instance))

(event `self.Box.OnComponentBeginOverlap`
  (params (OverlappedComponent :type "PrimitiveComponent Object Reference") (OtherActor :type "Actor Object Reference") (OtherComp :type "PrimitiveComponent Object Reference") (OtherBodyIndex :type Integer) (bFromSweep :type Boolean) (SweepResult :type "HitResult Structure (by ref)"))
  (if (== OtherActor (`GameplayStatics.GetPlayerCharacter` 0))
    (bind (_direction _alpha) (`Timeline|ButtonMovement`)
      (:`Update`
        (`SceneComponent.K2_SetRelativeLocation` (`self.Cube`) (`KismetMathLibrary.VLerp` (0.0 0.0 0.0) (0.0 0.0 100.0) _alpha) false false)
        (set `/Game/Miscellaneous/BP_GameInstance.IsBlueBtnPressed` true (`self.As BP Game Instance`))))))

(fn `UserConstructionScript`)