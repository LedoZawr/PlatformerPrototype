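; Base spline actor for rails that builds a chain of deformed meshes along its spline in the construction script.
; It divides spline length by a section length, optionally derived from actor X scale, with a flag restricting output to full-length sections.
; Each segment samples position and tangent by distance, clamping tangents to section length.
; Segments get configurable collision and a custom object channel.
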(fn `GetEndPosTangent`
  (params (Index :type Integer))
  (returns (Position :type "Vector Structure") (tangent :type "Vector Structure"))
  (bind _spline (`self.Spline`))
  (bind _returnvalue (* (+ Index 1) (`self.SectionLength`)))
  ;[1 1 1] Same as start pos but index +1 to get end pos
  (return (`SplineComponent.GetLocationAtDistanceAlongSpline` _spline _returnvalue "Local") (`KismetMathLibrary.ClampVectorSize` (`SplineComponent.GetTangentAtDistanceAlongSpline` _spline _returnvalue "Local") 0.0 (`self.SectionLength`))))

(fn `GetStartPosTangent`
  (params (Index :type Integer))
  (returns (Position :type "Vector Structure") (tangent :type "Vector Structure"))
  (bind _spline (`self.Spline`))
  (bind _returnvalue (* Index (`self.SectionLength`)))
  ;[1 1 1] Start Tangent at the loop index because for loop only indexes spline points
  (return (`SplineComponent.GetLocationAtDistanceAlongSpline` _spline _returnvalue "Local") (`KismetMathLibrary.ClampVectorSize` (`SplineComponent.GetTangentAtDistanceAlongSpline` _spline _returnvalue "Local") 0.0 (`self.SectionLength`))))

(fn `UserConstructionScript`
  (locals (LoopIndex :type Integer))
  (bind _returnvalue_x (`KismetMathLibrary.BreakVector` (`self.GetActorScale3D`)))
  (if (`self.AllowScaling?`)
    (set `self.SectionLength` (* _returnvalue_x 100.0)))
  (if (`self.MustBeFullLengthMeshes?`)
    (for _index (range (`KismetMathLibrary.FTrunc` (/ (`SplineComponent.GetSplineLength` (`self.Spline`)) (`self.SectionLength`))))
      (set `local.LoopIndex` _index)
      ;[1 1 1] returns selected mesh
      (bind _returnvalue (`AddComponent|NODE_AddSplineMeshComponent-0` :!label _label))
      (`StaticMeshComponent.SetStaticMesh` _returnvalue (`self.SplineMesh`))
      ;[1 1 1] Sets forward axis (depends on mesh local position)
      (`SplineMeshComponent.SetForwardAxis` _returnvalue "X" true)
      (bind (_position _tangent) (`self.GetStartPosTangent` (`local.LoopIndex`)))
      (bind (_position_2 _tangent_2) (`self.GetEndPosTangent` (`local.LoopIndex`)))
      (`SplineMeshComponent.SetStartAndEnd` _returnvalue _position _tangent _position_2 _tangent_2 true)
      (`PrimitiveComponent.SetCollisionEnabled` _returnvalue (`self.CollisionType`))
      (`PrimitiveComponent.SetCollisionObjectType` _returnvalue "ECC_GameTraceChannel2"))
    (else
      ;[1 1 1] Spline length divided by section lenght = amount of spline meshes
      (for _index_2 (range (+ (`KismetMathLibrary.FTrunc` (/ (`SplineComponent.GetSplineLength` (`self.Spline`)) (`self.SectionLength`))) 1))
        (set `local.LoopIndex` _index_2)
        (goto _label)))))