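; BP_FallBox is a trigger volume that kills the player when they fall into it.
; Tick caches the player character as a BP_Player reference until it is valid.
; When the box component is overlapped by player character 0, it calls FallDeath on that cached player.
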(event `self.ReceiveBeginPlay`)

(event `self.ReceiveTick`
  (params (DeltaSeconds :type "Float (single-precision)"))
  (`/Engine/EditorBlueprintResources/StandardMacros.IsValid` (`self.As BP Player`)
    (:`Is Not Valid`
      (bind _asbp_player (cast `/Game/Characters/BP_Player` (`GameplayStatics.GetPlayerCharacter` 0)))
      (set `self.As BP Player` _asbp_player))))

(event `self.Box.OnComponentBeginOverlap`
  (params (OverlappedComponent :type "PrimitiveComponent Object Reference") (OtherActor :type "Actor Object Reference") (OtherComp :type "PrimitiveComponent Object Reference") (OtherBodyIndex :type Integer) (bFromSweep :type Boolean) (SweepResult :type "HitResult Structure (by ref)"))
  (if (== OtherActor (`GameplayStatics.GetPlayerCharacter` 0))
    (`/Game/Characters/BP_Player.FallDeath` (`self.As BP Player`))))

(fn `UserConstructionScript`)