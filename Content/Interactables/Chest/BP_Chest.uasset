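; BP_Chest is an interactable chest that opens when the player character enters its box trigger and spawns its stored coins.
; A timeline rotates the lid, then a delayed while loop spawns BP_Coin actors one by one, calling CoinFromChest on each.
; Once empty, it destroys the treasure component and closes after a delay.
; Leaving the trigger reverses the lid, with boolean gates blocking re-opening and closing during coin spawning.
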(event `self.Box.OnComponentBeginOverlap`
  (params (OverlappedComponent :type "PrimitiveComponent Object Reference") (OtherActor :type "Actor Object Reference") (OtherComp :type "PrimitiveComponent Object Reference") (OtherBodyIndex :type Integer) (bFromSweep :type Boolean) (SweepResult :type "HitResult Structure (by ref)"))
  ;[1 1 1] Begin and end overlap events handle
  (if (== OtherActor (`GameplayStatics.GetPlayerCharacter` 0))
    (`self.Open Box`)))

(event `self.Box.OnComponentEndOverlap`
  (params (OverlappedComponent :type "PrimitiveComponent Object Reference") (OtherActor :type "Actor Object Reference") (OtherComp :type "PrimitiveComponent Object Reference") (OtherBodyIndex :type Integer))
  ;[1 1 1] Begin and end overlap events handle
  (if (== OtherActor (`GameplayStatics.GetPlayerCharacter` 0))
    (`self.Close Box`)))

(event `Open Box`
  ;[1 1 1] Booleans to prevent visual bugs
  (if (`self.CanLidOpen?`)
    (set `self.CanLidOpen?` false)
    ;[1 1 1] Opening the lid via timeline and relative rotation
    (bind (_direction _alpha) (`Timeline|Open_Lid` :!label _label)
      (:`Update`
        (`SceneComponent.K2_SetRelativeRotation` (`self.Lid`) (* (struct :`Roll` -120.0) _alpha) false false))
      (:`Finished`
        ;[1 1 1] Checking if amount of coins is more that zero and starting while loop to spawn all coins
        (if (> (`self.Amount of coins`) 0)
          (set `self.CanLidClose?` false)
          (`/Game/Interactables/Chest/BP_MacroLib.WhileLoopWithDelay` (> (`self.Amount of coins`) 0) 0.1
            (:`Loop Body`
              ;[1 1 1] Decrementing coin count, spawning actors and starting event from coin bp
              (`/Engine/EditorBlueprintResources/StandardMacros.DecrementInt` (`self.Amount of coins`)
                (:`  `
                  (bind _returnvalue (`|SpawnActorFromClass` "/Game/Interactables/Coin/BP_Coin.BP_Coin_C" (`KismetMathLibrary.MakeTransform` (`self.K2_GetActorLocation`)) "Undefined" "MultiplyWithRoot" null null))
                  (`/Game/Interactables/Coin/BP_Coin.CoinFromChest` _returnvalue))))
            (:`Completed`
              ;[1 1 1] Destroying treasure component and closing the box after delay
              (`ActorComponent.K2_DestroyComponent` (`self.Treasure`))
              (set `self.CanLidClose?` true)
              (`KismetSystemLibrary.Delay` 2.0)
              (`self.Close Box`))))))))

(event `Close Box`
  ;[1 1 1] Booleans to prevent visual bugs
  (if (`self.CanLidClose?`)
    (set `self.CanLidOpen?` true)
    (goto _label :!via `Reverse`)))

(fn `UserConstructionScript`)