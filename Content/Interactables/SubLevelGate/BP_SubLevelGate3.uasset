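; BP_SubLevelGate3 is a gate that teleports the player to another gate behind a screen fade.
; On BeginPlay it finds the BP_SubLevelGate actor and stores it as LvlGate2.
; When the player overlaps its Box, it plays a fade-in widget, swaps to a fade-out widget, and moves the player to that gate's SpawnLocation transform, using delays for timing.
; Unwired nodes for game-instance access and sublevel opening never run.
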(event `self.ReceiveBeginPlay`
  (bind _returnvalue (`GameplayStatics.GetActorOfClass` "/Game/Interactables/SubLevelGate/BP_SubLevelGate.BP_SubLevelGate_C"))
  (set `self.LvlGate2` _returnvalue))

(event `self.Box.OnComponentBeginOverlap`
  (params (OverlappedComponent :type "PrimitiveComponent Object Reference") (OtherActor :type "Actor Object Reference") (OtherComp :type "PrimitiveComponent Object Reference") (OtherBodyIndex :type Integer) (bFromSweep :type Boolean) (SweepResult :type "HitResult Structure (by ref)"))
  (if (== OtherActor (`GameplayStatics.GetPlayerCharacter` 0))
    (bind _returnvalue (`|CreateWidget` "/Game/Interactables/SubLevelGate/WB_SubLevelGateFadeIn.WB_SubLevelGateFadeIn_C"))
    (bind _output_get (set `self.FadeInWidget` _returnvalue))
    (`UserWidget.AddToViewport` _output_get 0)
    (`/Game/Interactables/SubLevelGate/WB_SubLevelGateFadeIn.PlayFadeIn` (`self.FadeInWidget`))
    (`KismetSystemLibrary.Delay` 0.5)
    (bind _returnvalue_2 (`|CreateWidget` "/Game/Interactables/SubLevelGate/WB_SubLevelGateFadeOut.WB_SubLevelGateFadeOut_C"))
    (bind _output_get_2 (set `self.FadeOutWidget` _returnvalue_2))
    (`UserWidget.AddToViewport` _output_get_2 0)
    (`Widget.RemoveFromParent` (`self.FadeInWidget`))
    (`self.K2_SetActorTransform` (`GameplayStatics.GetPlayerCharacter` 0) (`SceneComponent.K2_GetComponentToWorld` (`/Game/Interactables/SubLevelGate/BP_SubLevelGate.SpawnLocation` (`self.LvlGate2`))) false false)
    (`KismetSystemLibrary.Delay` 1.0)
    (`/Game/Interactables/SubLevelGate/WB_SubLevelGateFadeOut.PlayFadeOut` (`self.FadeOutWidget`))))

(fn `UserConstructionScript`)