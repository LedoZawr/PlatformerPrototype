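; BP_HealthPack is a health pickup that spins, bobs and flies toward the player when their health is not full.
; Tick caches the player reference, rotates the mesh and drives the bob timeline.
; MagnetCollision starts a timeline that pulls the actor in with VInterpTo, and PickUpCollision passes HealAmount to the player and destroys the pack.
; Both overlaps accept only the player and read health from the GameInstance.
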(event `self.ReceiveBeginPlay`
  (bind _asbp_game_instance (cast `/Game/Miscellaneous/BP_GameInstance` (`GameplayStatics.GetGameInstance`)))
  (set `self.As BP Game Instance` _asbp_game_instance))

(event `self.ReceiveTick`
  (params (DeltaSeconds :type "Float (single-precision)"))
  (`/Engine/EditorBlueprintResources/StandardMacros.IsValid` (`self.As BP Player`)
    (:`Is Valid`
      _)
    (:`Is Not Valid`
      (bind _asbp_player (cast `/Game/Characters/BP_Player` (`GameplayStatics.GetPlayerCharacter` 0)))
      (set `self.As BP Player` _asbp_player)))
  ;[1 1 1] Rotation and Up/Down movement
  (`SceneComponent.K2_AddRelativeRotation` (`self.HealthPack`) (`KismetMathLibrary.MakeRotator` 0.0 0.0 (`self.RotationSpeed`)) false false)
  (bind (_direction _up_down) (`Timeline|HealthUp/Down`)
    (:`Update`
      (`SceneComponent.K2_SetRelativeLocation` (`self.HealthPack`) (`KismetMathLibrary.VLerp` (0.0 0.0 0.0) (0.0 0.0 10.0) _up_down) false false))))

(event `self.MagnetCollision.OnComponentBeginOverlap`
  (params (OverlappedComponent :type "PrimitiveComponent Object Reference") (OtherActor :type "Actor Object Reference") (OtherComp :type "PrimitiveComponent Object Reference") (OtherBodyIndex :type Integer) (bFromSweep :type Boolean) (SweepResult :type "HitResult Structure (by ref)"))
  (bind _returnvalue_location (`KismetMathLibrary.BreakTransform` (`self.GetTransform`)))
  (bind _as_bp_game_instance (`self.As BP Game Instance`))
  ;[1 1 1] Health Magnet
  (if (and (== OtherActor (`GameplayStatics.GetPlayerCharacter` 0)) (!= (`/Game/Miscellaneous/BP_GameInstance.GIHeath` _as_bp_game_instance) (`/Game/Miscellaneous/BP_GameInstance.GIMaxHealth` _as_bp_game_instance)))
    (bind (_direction _traveltime) (`Timeline|TravelTime` :!via `PlayFromStart`)
      (:`Update`
        (`self.K2_SetActorLocation` (+ _traveltime (`KismetMathLibrary.VInterpTo` _returnvalue_location (`self.K2_GetActorLocation` (`GameplayStatics.GetPlayerCharacter` 0)) (`GameplayStatics.GetWorldDeltaSeconds`) 10.0)))))))

(event `self.PickUpCollision.OnComponentBeginOverlap`
  (params (OverlappedComponent :type "PrimitiveComponent Object Reference") (OtherActor :type "Actor Object Reference") (OtherComp :type "PrimitiveComponent Object Reference") (OtherBodyIndex :type Integer) (bFromSweep :type Boolean) (SweepResult :type "HitResult Structure (by ref)"))
  (bind _as_bp_game_instance (`self.As BP Game Instance`))
  (if (and (== OtherActor (`GameplayStatics.GetPlayerCharacter` 0)) (!= (`/Game/Miscellaneous/BP_GameInstance.GIHeath` _as_bp_game_instance) (`/Game/Miscellaneous/BP_GameInstance.GIMaxHealth` _as_bp_game_instance)))
    (`/Game/Characters/BP_Player.OnHealthPickUp` (`self.As BP Player`) (`self.HealAmount`))
    (`self.K2_DestroyActor`)))

(fn `UserConstructionScript`)