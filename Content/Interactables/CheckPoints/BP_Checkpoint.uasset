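; BP_Checkpoint is a checkpoint actor that updates the respawn transform when its trigger box is first overlapped.
; The Box overlap plays a 2D sound, then copies the RespawnLocation component's world transform into BP_GameMode's SpawnTransform.
; It then reveals the Niagara effect and sets IsActivated to block repeat activation.
; The overlap does not filter which actor entered the box.
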(event `self.Box.OnComponentBeginOverlap`
  (params (OverlappedComponent :type "PrimitiveComponent Object Reference") (OtherActor :type "Actor Object Reference") (OtherComp :type "PrimitiveComponent Object Reference") (OtherBodyIndex :type Integer) (bFromSweep :type Boolean) (SweepResult :type "HitResult Structure (by ref)"))
  (if (not (`self.IsActivated?`))
    (bind _returnvalue (`GameplayStatics.CreateSound2D` "/Game/Interactables/CheckPoints/Checkpint.Checkpint" 1.0 1.0 0.0 null))
    (`AudioComponent.Play` _returnvalue 0.0)
    (bind _asbp_game_mode (cast `/Game/Miscellaneous/BP_GameMode` (`GameplayStatics.GetGameMode`)))
    (set `/Game/Miscellaneous/BP_GameMode.SpawnTransform` (`SceneComponent.K2_GetComponentToWorld` (`self.Respawn location`)) _asbp_game_mode)
    (`SceneComponent.SetVisibility` (`self.Niagara`) true false)
    (set `self.IsActivated?` true)))

(fn `UserConstructionScript`)