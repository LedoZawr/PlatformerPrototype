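; Grapple point actor that tracks a player target and its own state for a grappling mechanic.
; Tick compares the target's distance to an activation range, using two DoOnce gates that reset each other so state updates fire only on crossing.
; Interface events set the target, which also updates state, and store a line-of-sight flag exposed by a getter.
; StateCheck broadcasts OnGrapplePointStateChanged only when the state actually changes.
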(event `self.ReceiveTick`
  (params (DeltaSeconds :type "Float (single-precision)"))
  ;[1 1 1] Checking distance between player and activation point
  (`/Engine/EditorBlueprintResources/StandardMacros.IsValid` (`self.TargetActor`)
    (:`Is Valid`
      (if (<= (`KismetMathLibrary.Vector_Distance` (`self.K2_GetActorLocation` (`self.TargetActor`)) (`self.K2_GetActorLocation`)) (`self.ActivationDistance`))
        (`/Engine/EditorBlueprintResources/StandardMacros.DoOnce` false :!label _label
          (:`Completed`
            (`/Game/Interactables/Grapple/Interfaces/BPI_GrapplePoint.UpdateGrapplePointState` "NewEnumerator0")
            (goto _label_2 :!via `Reset`)))
        (else
          (`/Engine/EditorBlueprintResources/StandardMacros.DoOnce` false :!label _label_2
            (:`Completed`
              (`/Game/Interactables/Grapple/Interfaces/BPI_GrapplePoint.UpdateGrapplePointState` "NewEnumerator2")
              (goto _label :!via `Reset`))))))
    (:`Is Not Valid`
      (`|ExecutionSequence`
        (:`then_0`
          (goto _label :!via `Reset`))
        (:`then_1`
          (goto _label_2 :!via `Reset`))))))

(event `/Game/Interactables/Grapple/Interfaces/BPI_GrapplePoint.SetIsInLineOfSight`
  (params (LineOfSight :type Boolean))
  ;[1 1 1] Interface functionality handle
  (set `self.IsInLineOfSight` LineOfSight))

(event `/Game/Interactables/Grapple/Interfaces/BPI_GrapplePoint.SetGrapplePontTarget`
  (params (Player :type "Actor Object Reference"))
  ;[1 1 1] Interface functionality handle
  (bind _output_get (set `self.TargetActor` Player))
  (`/Engine/EditorBlueprintResources/StandardMacros.IsValid` _output_get
    (:`Is Valid`
      (`self.UpdateGrapplePointState` "NewEnumerator0"))
    (:`Is Not Valid`
      (`self.UpdateGrapplePointState` "NewEnumerator2"))))

(event `/Game/Interactables/Grapple/Interfaces/BPI_GrapplePoint.UpdateGrapplePointState`
  (params (NewState :type "/Game/Interactables/Grapple/Enum_GrapplePointState Enum" :default "NewEnumerator0"))
  ;[1 1 1] Interface functionality handle
  (`self.StateCheck` NewState))

(fn `GetGrapplePointState`
  (returns (State :type "/Game/Interactables/Grapple/Enum_GrapplePointState Enum"))
  (return (`self.GrapplePointState`)))

(fn `GetLineOfSight`
  (returns (LineOfSight :type Boolean))
  (return (`self.IsInLineOfSight`)))

(fn `StateCheck`
  (params (NewPointState :type "/Game/Interactables/Grapple/Enum_GrapplePointState Enum" :default "NewEnumerator0"))
  (locals (L_PreviousState :type "/Game/Interactables/Grapple/Enum_GrapplePointState Enum"))
  (set `local.L_PreviousState` (`self.GrapplePointState`))
  (if (`|EnumInequality` NewPointState (`self.GrapplePointState`))
    (set `self.GrapplePointState` NewPointState)
    (`self.OnGrapplePointStateChanged` self (`self.GrapplePointState`))
    (else
      (set `self.GrapplePointState` (`local.L_PreviousState`)))))

(fn `UserConstructionScript`)