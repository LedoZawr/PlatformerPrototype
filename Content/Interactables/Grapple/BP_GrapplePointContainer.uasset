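; Grapple point container: a box trigger that hands grapple points to the player while it is inside.
; On begin overlap by a "Player"-tagged component, it gives every BP_GrapplePoint in the world, not just the box, that target and sends the player the list with an activation distance.
; End overlap clears the player's points, but empties its own array first, so point targets are never reset.
; GetLineOfSight is a stub returning false.
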(event `self.ReceiveBeginPlay`)

(event `self.Box.OnComponentBeginOverlap`
  (params (OverlappedComponent :type "PrimitiveComponent Object Reference") (OtherActor :type "Actor Object Reference") (OtherComp :type "PrimitiveComponent Object Reference") (OtherBodyIndex :type Integer) (bFromSweep :type Boolean) (SweepResult :type "HitResult Structure (by ref)"))
  (bind _outactors (`GameplayStatics.GetAllActorsOfClass` "/Game/Interactables/Grapple/BP_GrapplePoint.BP_GrapplePoint_C"))
  (set `self.GrapplePoints` _outactors)
  (if (`ActorComponent.ComponentHasTag` OtherComp "Player")
    (for _array_element (`self.GrapplePoints`)
      (message `/Game/Interactables/Grapple/Interfaces/BPI_GrapplePoint.SetGrapplePontTarget` _array_element OtherActor))
    (message `/Game/Interactables/Grapple/Interfaces/BPI_PlayerGrapple.SetPossibleGrapplePoints` OtherActor (`self.GrapplePoints`) 1800.0)))

(event `self.Box.OnComponentEndOverlap`
  (params (OverlappedComponent :type "PrimitiveComponent Object Reference") (OtherActor :type "Actor Object Reference") (OtherComp :type "PrimitiveComponent Object Reference") (OtherBodyIndex :type Integer))
  (`KismetArrayLibrary.Array_Clear` (`self.GrapplePoints`))
  (if (`ActorComponent.ComponentHasTag` OtherComp "Player")
    (for _array_element (`self.GrapplePoints`)
      (message `/Game/Interactables/Grapple/Interfaces/BPI_GrapplePoint.SetGrapplePontTarget` _array_element null))
    (message `/Game/Interactables/Grapple/Interfaces/BPI_PlayerGrapple.ClearAllGrapplePoints` OtherActor)))

(fn `GetLineOfSight`
  (returns (LineOfSight :type Boolean))
  (return false))

(fn `UserConstructionScript`)